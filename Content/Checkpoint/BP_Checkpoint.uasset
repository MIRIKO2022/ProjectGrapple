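; Checkpoint actor for a chained race course: only the active one, marked by a blinking neon material, responds to the first-person character's overlap.
; On trigger it records itself as the GameMode's LastCheckpoint, plays a sound, then activates NextCheckpoint and destroys itself.
; Without a valid next checkpoint, it stops the HUD timer, shows both Lose and Win widgets with UI-only input, and runs a development-only pause-and-quit WinGame event.
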(event OnComponentBeginOverlap(Trigger)
  (params (OverlappedComponent :type Primitive%20Component%20Object%20Reference) (OtherActor :type Actor%20Object%20Reference) (OtherComp :type Primitive%20Component%20Object%20Reference) (OtherBodyIndex :type Integer) (bFromSweep :type Boolean) (SweepResult :type Hit%20Result%20Structure%20%28by%20ref%29))
  (bind _returnvalue (Game|GetPlayerController 0))
  ;[0.15 0.15 0.15 0.5] Collision logic
  (Utilities|Casting|CastToBP_FirstPersonCharacter OtherActor)
  (if (Variables|Default|GetbIsActive)
    (bind _asbp_first_person_game_mode (Utilities|Casting|CastToBP_FirstPersonGameMode (Game|GetGameMode)))
    (Variables|/Game/FirstPerson/Blueprints/BP_FirstPersonGameMode.BP_FirstPersonGameMode_C|Setlast%20checkpoint _asbp_first_person_game_mode self)
    (Audio|PlaySound2D "/Game/Checkpoint/sonic-checkpoint.sonic-checkpoint" 1.0 1.0 0.0 0 0)
    (Utilities|IsValid (Variables|Default|GetNextCheckpoint)
      (:Is%20Valid
        (CallFunction|ActiveCheckpoint (Variables|Default|GetNextCheckpoint))
        (Actor|DestroyActor))
      (:Is%20Not%20Valid
        (bind _asbp_first_person_character (Utilities|Casting|CastToBP_FirstPersonCharacter OtherActor))
        (Variables|/Game/UI/WidgetBlueprint/WBP_HUD.WBP_HUD_C|SetIsTimerActive (Variables|/Game/FirstPerson/Blueprints/BP_FirstPersonCharacter.BP_FirstPersonCharacter_C|GetMyHUD _asbp_first_person_character) false)
        (bind _asbp_first_person_character_2 (Utilities|Casting|CastToBP_FirstPersonCharacter (Game|GetPlayerCharacter 0)))
        (Widget|RemovefromParent (Variables|/Game/FirstPerson/Blueprints/BP_FirstPersonCharacter.BP_FirstPersonCharacter_C|GetMyHUD _asbp_first_person_character_2))
        (bind _returnvalue_2 (UserInterface|CreateWidget "/Game/UI/WidgetBlueprint/WBP_Lose.WBP_Lose_C"))
        (UserInterface|Viewport|AddtoViewport _returnvalue_2 0)
        (Variables|/Script/Engine.PlayerController|SetbShowMouseCursor _returnvalue true)
        (Input|SetInputModeUIOnly _returnvalue _returnvalue_2 "LockAlways" false)
        (bind _returnvalue_3 (UserInterface|CreateWidget "/Game/UI/WidgetBlueprint/WBP_Win.WBP_Win_C"))
        (UserInterface|Viewport|AddtoViewport _returnvalue_3 0)
        (CallFunction|WinGame)))))

(event Custom|ActiveCheckpoint
  ;[0.15 0.15 0.15 0.5] Active Next Checkpoint logic
  (Variables|Default|SetbIsActive true)
  (Rendering|Material|SetMaterial (Variables|Default|GetStaticMesh) 0 "/Game/NeonGlowMaterials/Materials/Instances/NeonBlinkColor/MI_Neon_Blink_08.MI_Neon_Blink_08"))

(event Custom|Win%20Game
  ;[0.15 0.15 0.15 0.5] End Game (Development only)
  (Game|SetGamePaused true)
  (Development|PrintString "YOU WIN" true true "(R=0.053603,G=1.000000,B=0.000000,A=1.000000)")
  (Utilities|FlowControl|Delay 5.0)
  (Game|QuitGame 0 "Quit" false))

(event EventBeginPlay
  ;[0.15 0.15 0.15 0.5] Blinking logic
  (if (Variables|Default|GetbIsActive)
    (Rendering|Material|SetMaterial (Variables|Default|GetStaticMesh) 0 "/Game/NeonGlowMaterials/Materials/Instances/NeonBlinkColor/MI_Neon_Blink_08.MI_Neon_Blink_08")))

(fn ConstructionScript)